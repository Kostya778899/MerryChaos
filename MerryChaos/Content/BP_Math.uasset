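; BP_Math provides a float helper, FloatBringUp, that snaps an input to one of three supplied values.
; An input equal to Middle returns Middle, one below returns Min, and one above returns Max.
; The function uses chained exact comparisons with no tolerance or interpolation, so it acts as a three-way step around Middle.
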(fn `FloatBringUp`
  (params (`Value(Input)` :type "Float (double-precision)") (Middle :type "Float (double-precision)") (Min :type "Float (double-precision)" :default -1.0) (Max :type "Float (double-precision)" :default 1.0))
  (returns (`Value(Output)` :type "Float (double-precision)"))
  (if (== `Value(Input)` Middle)
    (return (`local.Middle`))
    (elif (< `Value(Input)` Middle)
      (return (`local.Min`))
      (elif (> `Value(Input)` Middle)
        (return (`local.Max`))))))