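; Player character Blueprint that moves from joystick axis input and turns to face its direction of travel.
; JoystickX adds movement along the control rotation's forward vector and JoystickY along its right vector.
; Each Tick sets the actor's rotation directly to a look-at toward its location plus velocity, with no interpolation or axis filtering.
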(event `self.ReceiveTick`
  (params (DeltaSeconds :type "Float (single-precision)"))
  (bind _returnvalue (`self.K2_GetActorLocation`))
  (`self.K2_SetActorRotation` (`KismetMathLibrary.FindLookAtRotation` _returnvalue (+ _returnvalue (`self.GetVelocity`)))))

(event `InputAxis|JoystickX`
  (params (AxisValue :type "Float (single-precision)"))
  ;[1 1 1] MoveXY
  (`self.AddMovementInput` (`KismetMathLibrary.GetForwardVector` (`self.GetControlRotation`)) AxisValue))

(event `InputAxis|JoystickY`
  (params (AxisValue :type "Float (single-precision)"))
  ;[1 1 1] MoveXY
  (`self.AddMovementInput` (`KismetMathLibrary.GetRightVector` (`self.GetControlRotation`)) AxisValue))

(fn `UserConstructionScript`)