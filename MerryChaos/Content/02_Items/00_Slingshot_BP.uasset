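; Slingshot actor that previews a touch-aimed shot trajectory; it does not spawn or fire a projectile.
; Every tick, the screen offset between the first touch and the projected ShootPoint becomes an X/Z-plane velocity, with X inverted and scaled by ShotStrength.
; A predicted projectile path from ShootPoint is debug-drawn, regardless of press state.
; Touch events record press state and start position, both unused here, and print debug positions.
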(event `self.ReceiveTick`
  (params (DeltaSeconds :type "Float (single-precision)"))
  (bind _returnvalue (`GameplayStatics.GetPlayerController` 0))
  (bind (_locationx _locationy) (`PlayerController.GetInputTouchState` _returnvalue "Touch1"))
  (bind (_returnvalue_x _returnvalue_y) (`KismetMathLibrary.BreakVector2D` (- (`KismetMathLibrary.MakeVector2D` _locationx _locationy) (`GameplayStatics.ProjectWorldToScreen` _returnvalue (`SceneComponent.K2_GetComponentLocation` (`self.ShootPoint`))))))
  (`GameplayStatics.Blueprint_PredictProjectilePath_ByTraceChannel` :`StartPos` (`SceneComponent.K2_GetComponentLocation` (`self.ShootPoint`)) :`LaunchVelocity` (* (`KismetMathLibrary.MakeVector` (* _returnvalue_x -1.0) 0.0 _returnvalue_y) (`self.ShotStrength`)) :`ProjectileRadius` 5.0 :`DrawDebugType` "ForDuration" :`DrawDebugTime` 0.0 :`SimFrequency` 25.0 :`MaxSimTime` 5.0))

(event `InputTouch`
  (params (Location :type "Vector Structure") (FingerIndex :type "ETouchIndex Enum"))
  (:`Pressed`
    (set `self.IsPressed` true)
    (set `self.StartClickPosition` (`KismetMathLibrary.Conv_VectorToVector2D` Location))
    (`KismetSystemLibrary.PrintString` (`KismetStringLibrary.Conv_VectorToString` Location) true true (struct :`G` 0.66 :`B` 1.0 :`A` 1.0) 100.0)
    (`KismetSystemLibrary.PrintString` (`KismetStringLibrary.Conv_Vector2dToString` (`GameplayStatics.ProjectWorldToScreen` (`GameplayStatics.GetPlayerController` 0) (`SceneComponent.K2_GetComponentLocation` (`self.ShootPoint`)))) true true (struct :`G` 0.66 :`B` 1.0 :`A` 1.0) 100.0))
  (:`Released`
    (set `self.IsPressed` false)))

(fn `UserConstructionScript`)