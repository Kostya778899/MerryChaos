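; Slingshot weapon actor, apparently an unfinished prototype of touch-driven drag-to-aim shooting.
; Cursor-over events track hovering, and a touch press on the slingshot switches its shoot state, with debug prints reporting both.
; Touch release only clears the pressed flag and prints state.
; Disconnected logic would predict a projectile arc from the screen-space drag relative to ShootPoint, scaled by ShotStrength, but nothing runs it or fires a projectile.
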(event `self.ReceiveBeginPlay`)

(event `self.ReceiveTick`
  (params (DeltaSeconds :type "Float (single-precision)"))
  (`KismetSystemLibrary.PrintString` (`KismetStringLibrary.Conv_BoolToString` (`self.IsCursorBegin`)) true true (struct :`G` 0.66 :`B` 1.0 :`A` 1.0) 0.0))

(event `self.ReceiveActorBeginCursorOver`
  (set `self.IsCursorBegin` true)
  (`KismetSystemLibrary.PrintString` (`KismetStringLibrary.Conv_BoolToString` (`self.IsCursorBegin`)) :!label _label))

(event `self.ReceiveActorEndCursorOver`
  (set `self.IsCursorBegin` false)
  (goto _label))

(event `InputTouch`
  (params (Location :type "Vector Structure") (FingerIndex :type "ETouchIndex Enum"))
  (:`Pressed`
    (set `self.IsPressed` true)
    (if (and (`|EnumEquality` (`self.ShootState`) "NewEnumerator3") (`self.IsCursorBegin`))
      (set `self.ShootState` "NewEnumerator0")
      (`KismetSystemLibrary.PrintString` (`|GetEnumeratorNameAsString` (`self.ShootState`)))))
  (:`Released`
    (set `self.IsPressed` false)
    (`KismetSystemLibrary.PrintString` (`KismetStringLibrary.Concat_StrStr` (`KismetStringLibrary.Conv_BoolToString` (`|EnumEquality` (`self.ShootState`) "NewEnumerator0")) "                    " (`KismetStringLibrary.Conv_BoolToString` (`self.IsCursorBegin`))))))

(fn `UserConstructionScript`)